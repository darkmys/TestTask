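; Spawner Blueprint that scatters actors from a class array at random points inside a Box, with random rotation and per-axis scale.
; Spawn creates a batch of each class and sets a flag; while the flag is set, it calls Transform to re-randomize rotation and scale instead.
; Clear destroys actors and resets the flag.
; Clear and Transform find actors by class level-wide, not through stored references.
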(event `Clear`
  (for _array_element (`self.StaticMesh`)
    (bind _outactors (`GameplayStatics.GetAllActorsOfClass` _array_element))
    (`self.K2_DestroyActor` _outactors)
    (set `self.Condition` false)))

(event `Spawn`
  (bind (_returnvalue_roll _returnvalue_pitch _returnvalue_yaw) (`KismetMathLibrary.BreakRotator` (`KismetMathLibrary.RandomRotator` false)))
  (bind _returnvalue (`KismetMathLibrary.RandomFloatInRange` 0.1 1.0))
  (bind _box (`self.Box`))
  (if (`self.Condition`)
    (`self.Transform`)
    (else
      (for _ (range (+ (`self.Last Index`) 1))
        (for _array_element (`self.StaticMesh`)
          (`|SpawnActorFromClass` _array_element (`KismetMathLibrary.MakeTransform` (`KismetMathLibrary.RandomPointInBoundingBox` (`SceneComponent.RelativeLocation` _box) (`BoxComponent.GetScaledBoxExtent` _box)) (`KismetMathLibrary.MakeRotator` _returnvalue_roll _returnvalue_pitch _returnvalue_yaw) (`KismetMathLibrary.MakeVector` _returnvalue _returnvalue _returnvalue)) "AdjustIfPossibleButDontSpawnIfColliding" "MultiplyWithRoot" null null)
          (set `self.Condition` true))))))

(event `Transform`
  (bind _returnvalue (`KismetMathLibrary.RandomFloatInRange` 0.1 1.0))
  (bind _staticmesh (`self.StaticMesh`))
  (for (_ _array_index) _staticmesh
    (bind _outactors (`GameplayStatics.GetAllActorsOfClass` (`|GetArrayItem` _staticmesh _array_index)))
    (for _array_element _outactors
      (`self.K2_SetActorRotation` _array_element (`KismetMathLibrary.RandomRotator` false) false)
      (`self.SetActorScale3D` _array_element (`KismetMathLibrary.MakeVector` _returnvalue _returnvalue _returnvalue)))))

(fn `UserConstructionScript`)